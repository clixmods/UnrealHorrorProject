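; Horror prop actor that moves its static mesh to a random spline point while the player is not looking at it.
; Each tick, IsOnScreen projects the location to the player's viewport with a top-left margin, ignoring projection success and occlusion.
; When the mesh is off screen, it teleports to a TeleportPoint spline point that is also off screen.
; IsTped limits this to one move until the mesh is seen again.
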(event `self.ReceiveTick`
  (params (DeltaSeconds :type "Float (single-precision)"))
  (bind _teleportpoint (`self.TeleportPoint`))
  (bind _result (`self.IsOnScreen` (`SceneComponent.K2_GetComponentLocation` (`self.StaticMesh`))))
  (if _result
    (set `self.IsTped` false)
    (elif (not (`self.IsTped`))
      (bind _output_get (set `self.NextLocation` (`SplineComponent.GetLocationAtSplinePoint` _teleportpoint (`KismetMathLibrary.RandomIntegerInRange` 0 (`SplineComponent.GetNumberOfSplinePoints` _teleportpoint)) "World")))
      (bind _result_2 (`self.IsOnScreen` _output_get))
      (if (not _result_2)
        (`SceneComponent.K2_SetWorldLocation` (`self.StaticMesh`) (`self.NextLocation`) false true)
        (`KismetSystemLibrary.PrintString` "Objet moving")
        (set `self.IsTped` true)))))

(fn `IsOnScreen`
  (params (Location :type "Vector Structure"))
  (returns (result :type Boolean))
  (bind (_returnvalue_x _returnvalue_y) (`KismetMathLibrary.BreakVector2D` (`WidgetLayoutLibrary.GetViewportSize`)))
  (bind _screenlocation (`PlayerController.ProjectWorldLocationToScreen` (`PlayerState.GetPlayerController` (`Pawn.PlayerState` (`GameplayStatics.GetPlayerPawn` 0))) Location true))
  (return (and (> (`KismetMathLibrary.BreakVector2D` _screenlocation) -300.0) (> (`.Y` (`KismetMathLibrary.BreakVector2D` _screenlocation)) -300.0) (< (`KismetMathLibrary.BreakVector2D` _screenlocation) _returnvalue_x) (< (`.Y` (`KismetMathLibrary.BreakVector2D` _screenlocation)) _returnvalue_y) true)))

(fn `UserConstructionScript`)