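; BP_PointLightFlick is a horror-content light that flickers by randomly varying its intensity.
; BeginPlay caches the light component's starting intensity as the base value.
; Tick accumulates delta time and, each time it reaches Delay, sets a random intensity within FlickVariation either side of that base, then resets the timer.
; The change is an instant step with no interpolation, and randomness stays centred on the original brightness.
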(event `self.ReceiveBeginPlay`
  (set `self.BaseIntensity` (`LightComponentBase.Intensity` (`self.LightComponent`))))

(event `self.ReceiveTick`
  (params (DeltaSeconds :type "Float (single-precision)"))
  (bind _output_get (set `self.currentDelay` (+ DeltaSeconds (`self.currentDelay`))))
  (if (>= _output_get (`self.Delay`))
    (`LightComponent.SetIntensity` (`self.LightComponent`) (`KismetMathLibrary.RandomFloatInRange` (- (`self.BaseIntensity`) (`self.FlickVariation`)) (+ (`self.BaseIntensity`) (`self.FlickVariation`))))
    (set `self.currentDelay` 0.0)))

(fn `UserConstructionScript`)