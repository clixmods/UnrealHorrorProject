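; Spot light Blueprint that makes its intensity flicker randomly around the value it has at BeginPlay.
; Tick accumulates time and, each time Delay is reached, picks a new random target within FlickVariation of that base intensity.
; On other frames it lerps the current intensity toward the target using DeltaSeconds as alpha, so the light drifts gradually instead of snapping.
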(event `self.ReceiveTick`
  (params (DeltaSeconds :type "Float (single-precision)"))
  (bind _lightcomponent (`self.LightComponent`))
  (bind _output_get (set `self.currentDelay` (+ (`self.currentDelay`) DeltaSeconds)))
  (if (>= _output_get (`self.Delay`))
    (bind _output_get_2 (set `self.TargetValue` (`KismetMathLibrary.RandomFloatInRange` (- (`self.BaseIntensity`) (`self.FlickVariation`)) (+ (`self.BaseIntensity`) (`self.FlickVariation`)))))
    (set `self.currentDelay` 0.0)
    (else
      (`LightComponent.SetIntensity` _lightcomponent (`KismetMathLibrary.Lerp` (`LightComponentBase.Intensity` _lightcomponent) _output_get_2 DeltaSeconds)))))

(event `self.ReceiveBeginPlay`
  (set `self.BaseIntensity` (`LightComponentBase.Intensity` (`self.LightComponent`))))

(fn `UserConstructionScript`)