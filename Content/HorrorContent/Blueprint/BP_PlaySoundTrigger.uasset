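; Trigger actor for the horror content that plays a configurable sound at its own location when its TriggerSound component is overlapped.
; Each play clears IsReplayable and resets a timer, which Tick accumulates and prints to screen until it exceeds TimeDelay.
; The trigger then either re-arms when CanReplaying is set or destroys itself.
; The FirstTime branch has no effect.
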(event `self.ReceiveBeginPlay`)

(event `self.ReceiveTick`
  (params (DeltaSeconds :type "Float (single-precision)"))
  (if (`self.IsReplayable`)
    _
    (elif (> (`self.currentTimeDelay`) (`self.TimeDelay`))
      (if (`self.firstTime`)
        _
        (else
          _))
      (if (`self.CanReplaying`)
        (set `self.IsReplayable` true)
        (else
          (`self.K2_DestroyActor`)))
      (else
        (bind _output_get (set `self.currentTimeDelay` (+ DeltaSeconds (`self.currentTimeDelay`))))
        (`KismetSystemLibrary.PrintString` (`KismetStringLibrary.Conv_DoubleToString` _output_get))))))

(event `self.TriggerSound.OnComponentBeginOverlap`
  (params (OverlappedComponent :type "PrimitiveComponent Object Reference") (OtherActor :type "Actor Object Reference") (OtherComp :type "PrimitiveComponent Object Reference") (OtherBodyIndex :type Integer) (bFromSweep :type Boolean) (SweepResult :type "HitResult Structure (by ref)"))
  (if (`self.IsReplayable`)
    (`GameplayStatics.PlaySoundAtLocation` (`self.Sound`) (`self.K2_GetActorLocation`) (struct) (`self.Volume Multiplier`) (`self.Pitch Multiplier`) (`self.Start Time`) (`self.Attenuation Settings`) (`self.Concurrency Settings`) null (`self.Initial Params`))
    (set `self.currentTimeDelay` 0.0)
    (set `self.IsReplayable` false)))

(fn `UserConstructionScript`)